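; AC_ItemComponent is an actor component that makes its owning actor a pickup item for the inventory system.
; On Interact, it passes its item row name and quantity to the interacting character's inventory component and destroys the owning actor if the add succeeds.
; It prints a debug message when that inventory is invalid, and an unconnected node for enabling owner replication never runs.
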(event `self.ReceiveBeginPlay`
  ;[1 1 1] dude i dunno... it doesnt work for me
)

(event `/Game/Modules/Interact/BPI_Interact.Interact`
  (params (CharacterRef :type "/Game/Modules/Core/ThirdPersonControl/Blueprints/BP_ThirdPersonCharacter Object Reference"))
  (bind _ac_inventorysystem (`/Game/Modules/Core/ThirdPersonControl/Blueprints/BP_ThirdPersonCharacter.AC_InventorySystem` CharacterRef))
  (bind (_itemid_datatable _itemid_rowname) (break `DataTableRowHandle` (`self.ItemID`)))
  (`/Engine/EditorBlueprintResources/StandardMacros.IsValid` _ac_inventorysystem
    (:`Is Valid`
      (bind _bsuccess (`/Game/Modules/Inventory/AC_InventorySystem.Add Item` _ac_inventorysystem _itemid_rowname (`self.Quantity`)))
      (if _bsuccess
        (`Actor.K2_DestroyActor` (`self.GetOwner`))))
    (:`Is Not Valid`
      (`KismetSystemLibrary.PrintString` "Not Valid"))))