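; Inventory component that stores items as a fixed-size array of item ID and quantity slots.
; Adding fills existing stacks one unit at a time up to the DT_Items max stack size, then uses empty slots.
; It also removes items, splits stacks and swaps differing items within or between inventories through a server event.
; Changes trigger a multicast update that calls OnUpdated, and P prints the contents for debugging.
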(event `self.ReceiveBeginPlay`
  (`KismetArrayLibrary.Array_Resize` (`self.Content`) (`self.Size`)))

(event `MC_Update`
  (`self.OnUpdated`))

(event `Server_SwitchSlots`
  (params (FromInventory :type "/Game/Modules/Inventory/AC_InventorySystem Object Reference") (`From Index` :type Integer) (`To Index` :type Integer))
  (`self.Switch Slots` FromInventory `From Index` `To Index`))

(event `Key|P`
  (params (Key :type "Key Structure"))
  (:`Pressed`
    (`self.Print Content`)))

(fn `Add Item`
  (params (ItemID :type Name) (Quantity :type Integer))
  (returns (bSuccess :type Boolean) (QuantityRemaining :type Integer))
  (locals (Local_QuantityRemaining :type Integer) (bFailed :type Boolean))
  (if (== ItemID "notInventory")
    (return false 0)
    (else
      (set `local.Local_QuantityRemaining` Quantity)
      (while (and (> (`local.Local_QuantityRemaining`) 0) (not (`local.bFailed`)))
        (bind (_index _bfound) (`self.Find Slot` (`local.ItemID`)))
        (if _bfound
          (`self.Add To Stack` _index 1)
          (`/Engine/EditorBlueprintResources/StandardMacros.DecrementInt` (`local.Local_QuantityRemaining`))
          (elif (`self.Empty Slots Available`)
            (bind _bcreated (`self.Create New Stack` (`local.ItemID`) 1))
            (if _bcreated
              (`/Engine/EditorBlueprintResources/StandardMacros.DecrementInt` (`local.Local_QuantityRemaining`))
              (else
                (set `local.bFailed` true)))
            (else
              (set `local.bFailed` true)))))
      (`self.MC_Update`)
      (return (not (`local.bFailed`)) (`local.Local_QuantityRemaining`)))))

(fn `Add To Stack`
  (params (Index :type Integer) (Quantity :type Integer))
  (bind (_output_itemid _output_quantity) (break `/Game/Modules/Inventory/S_Slot` (`|GetArrayItem` (`self.Content`) Index)))
  (`KismetArrayLibrary.Array_Set` (`self.Content`) Index (make `/Game/Modules/Inventory/S_Slot` _output_itemid (+ _output_quantity (`local.Quantity`)))))

(fn `Create New Stack`
  (params (ItemID :type Name) (Quantity :type Integer))
  (returns (bCreated :type Boolean))
  (bind (_bhasemptyslots _index) (`self.Empty Slots Available`))
  (if _bhasemptyslots
    (`KismetArrayLibrary.Array_Set` (`self.Content`) _index (make `/Game/Modules/Inventory/S_Slot` ItemID Quantity))
    (return true)
    (else
      (return false))))

(fn `Empty Slots Available`
  (returns (bHasEmptySlots :type Boolean) (Index :type Integer))
  (for (_array_element _array_index) (`self.Content`)
    (if (== (`.Quantity_5_F75D1B424A45C55595A003BFD5691FA5` (break `/Game/Modules/Inventory/S_Slot` _array_element)) 0)
      (return true _array_index)))
  (return false -1))

(fn `Find Slot`
  (params (ItemID :type Name))
  (returns (Index :type Integer) (bFound :type Boolean))
  (for _array_element (`self.Content`)
    (bind (_itemid _quantity) (break `/Game/Modules/Inventory/S_Slot` _array_element))
    (if (and (== _itemid ItemID) (< _quantity (`self.Get Max Stack Size` ItemID)))
      (return 0 true)))
  (return -1 false))

(fn `Get Max Stack Size`
  (params (ItemID :type Name))
  (returns (MaxStackSize :type Integer))
  (bind _returnvalue (`|GetDataTableRow` "/Game/Data/DT_Items.DT_Items" ItemID)
    (:`then`
      (return (`.MaxStackSize_14_F1A9A69C4A4CE0A05D28018F8DB830E2` (break `/Game/Modules/Inventory/S_Item` _returnvalue))))
    (:`RowNotFound`
      (return -1))))

(fn `Print Content`
  (for (_array_element _array_index) (`self.Content`)
    (bind (_itemid _quantity) (break `/Game/Modules/Inventory/S_Slot` _array_element))
    (`KismetSystemLibrary.PrintString` (`KismetStringLibrary.Concat_StrStr` (`KismetStringLibrary.Conv_IntToString` _array_index) ": " (`KismetStringLibrary.Conv_NameToString` _itemid) " = " (`KismetStringLibrary.Conv_IntToString` _quantity)))))

(fn `Remove Item`
  (params (Index :type Integer))
  (if (and (>= Index 0) (< Index (`KismetArrayLibrary.Array_Length` (`self.Content`))))
    (`KismetArrayLibrary.Array_Set` (`self.Content`) (`local.Index`))
    (`self.MC_Update`)))

(fn `Split Stack`
  (params (Index :type Integer) (Quantity :type Integer))
  (bind (_output_itemid _output_quantity) (break `/Game/Modules/Inventory/S_Slot` (`|GetArrayItem` (`self.Content`) Index)))
  (bind _returnvalue (- _output_quantity (`local.Quantity`)))
  (if (!= Quantity 0)
    (bind _bcreated (`self.Create New Stack` _output_itemid (`local.Quantity`)))
    (if _bcreated
      (if (== _returnvalue 0)
        (`self.Remove Item` (`local.Index`))
        (else
          (`KismetArrayLibrary.Array_Set` (`self.Content`) (`local.Index`) (make `/Game/Modules/Inventory/S_Slot` _output_itemid _returnvalue))))
      (`self.MC_Update`))))

(fn `Switch Slots`
  (params (FromInventory :type "/Game/Modules/Inventory/AC_InventorySystem Object Reference") (`From Index` :type Integer) (`To Index` :type Integer))
  (locals (`Local Slot` :type "/Game/Modules/Inventory/S_Slot Structure"))
  (bind _output_itemid (break `/Game/Modules/Inventory/S_Slot` (`|GetArrayItem` (`self.Content`) (`local.To Index`))))
  (set `local.Local Slot` (`|GetArrayItem` (`/Game/Modules/Inventory/AC_InventorySystem.Content` FromInventory) `From Index`))
  ;[1 1 1] check on other sources
  (if (not (< `To Index` 0))
    ;[1 1 1] check if we need to stack same items or swap them
    (if (not (== (`.ItemID_2_D60E2CC54C1375B10A7637A1B2AEE97A` (break `/Game/Modules/Inventory/S_Slot` (`local.Local Slot`))) _output_itemid))
      (`KismetArrayLibrary.Array_Set` (`/Game/Modules/Inventory/AC_InventorySystem.Content` (`local.FromInventory`)) (`local.From Index`) (`|GetArrayItem` (`self.Content`) (`local.To Index`)))
      (`KismetArrayLibrary.Array_Set` (`self.Content`) (`local.To Index`) (`local.Local Slot`))
      (`self.MC_Update`)
      (`self.MC_Update` (`local.FromInventory`)))))