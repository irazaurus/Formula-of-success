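; BP_Sky is a sky actor that runs a looping day-night cycle.
; Tick advances a 24-hour Time value at a rate set by Duration (real seconds per game hour), resetting it to zero at 24.
; Time maps to pitch on the sun and moon directional lights, held 180 degrees apart.
; The FogDencity curve, sampled at Time, drives the exponential height fog density.
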(event `self.ReceiveTick`
  (params (DeltaSeconds :type "Float (single-precision)"))
  (set `self.Time` (+ (/ DeltaSeconds (`self.Duration`)) (`self.Time`)))
  (if (>= (`self.Time`) 24.0)
    (set `self.Time` 0.0)
    (else
      ;[1 0.6483 0.3049] Sun rotation
      (`SceneComponent.K2_SetRelativeRotation` (`self.DirectionalLight_Sun`) (`KismetMathLibrary.MakeRotator` 0.0 (* (/ (`self.Time`) 24.0) 360.0)) false false)
      ;[0.2047 0.1752 1] Moon rotation
      (`SceneComponent.K2_SetRelativeRotation` (`self.DirectionalLight_Moon`) (`KismetMathLibrary.MakeRotator` 0.0 (+ (* (/ (`self.Time`) 24.0) 360.0) 180.0)) false false)
      (`ExponentialHeightFogComponent.SetFogDensity` (`self.ExponentialHeightFog`) (`CurveFloat.GetFloatValue` (`self.FogDencity`) (`self.Time`))))))

(fn `UserConstructionScript`)