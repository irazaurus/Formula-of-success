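; Store component that manages a coin budget, a buy inventory for player purchases and a sell inventory of goods for customers.
; Buying checks item cost against the budget, moves the item into an empty player slot via ServerSwitchSlots, then deducts coins.
; UpdateStock simulates daily sales from DT_Events, selling must-have items before maybe items within a per-day count and crediting the budget.
; It also hard-codes a lantern restock on one day.
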(fn `Add Coins`
  (params (Num :type Integer))
  (set `self.Budget` (+ Num (`self.Budget`))))

(fn `Add Item`
  (params (ItemID :type Name) (bSellItem :type Boolean))
  (if bSellItem
    (`/Game/Modules/Inventory/AC_InventorySystem.Add Item` (`self.SellInventory`) (`local.ItemID`) 1)
    (else
      (`/Game/Modules/Inventory/AC_InventorySystem.Add Item` (`self.BuyInventory`) (`local.ItemID`) 1))))

(fn `Buy Item`
  (params (Index :type Integer))
  (bind (_bcanbuy _cost) (`self.Can Buy Item` Index))
  (if _bcanbuy
    (bind _asbp_third_person_character (cast `/Game/Modules/Core/ThirdPersonControl/Blueprints/BP_ThirdPersonCharacter` (`GameplayStatics.GetPlayerCharacter` 0)))
    (bind _ac_inventorysystem (`/Game/Modules/Core/ThirdPersonControl/Blueprints/BP_ThirdPersonCharacter.AC_InventorySystem` _asbp_third_person_character))
    (bind (_bhasemptyslots _index) (`/Game/Modules/Inventory/AC_InventorySystem.Empty Slots Available` _ac_inventorysystem))
    (if _bhasemptyslots
      (`/Game/Modules/Inventory/AC_InventorySystem.Server_SwitchSlots` _ac_inventorysystem (`self.BuyInventory`) (`local.Index`) _index)
      (`self.Remove Coins` _cost))
    (else
      (return))))

(fn `Can Buy Item`
  (params (Index :type Integer))
  (returns (bCanBuy :type Boolean) (Cost :type Integer))
  (bind _buyinventory (`self.BuyInventory`))
  (bind _output_itemid (break `/Game/Modules/Inventory/S_Slot` (`|GetArrayItem` (`/Game/Modules/Inventory/AC_InventorySystem.Content` _buyinventory) Index)))
  (bind (_data_isingredient _data_ispotion _data_name _data_description _data_thumbnail _data_class _data_maxstacksize _data_cost) (break `/Game/Modules/Inventory/S_Item` (`/Game/Modules/Inventory/AC_InventorySystem.Get Item Data` _buyinventory _output_itemid)))
  (return (>= (`self.Budget`) _data_cost) _data_cost))

(fn `Remove Coins`
  (params (Num :type Integer))
  (set `self.Budget` (- (`self.Budget`) Num)))

(fn `Remove Item`
  (params (Index :type Integer) (bSellItem :type Boolean))
  (if bSellItem
    (`/Game/Modules/Inventory/AC_InventorySystem.Remove Item` (`self.SellInventory`) (`local.Index`))
    (else
      (`/Game/Modules/Inventory/AC_InventorySystem.Remove Item` (`self.BuyInventory`) (`local.Index`)))))

(fn `Update Stock`
  (params (Day :type Name))
  (locals (LocalLeftToBuy :type Integer) (LocalMustHaves :type Integer) (LocalMaybe :type Integer))
  (if (== Day "3")
    (`self.Add Item` "lantern"))
  (bind _returnvalue (`|GetDataTableRow` "/Game/Data/DT_Events.DT_Events" Day)
    (:`then`
      (bind (_name _items_num _musthave_items_id _maybe_items_id) (break `/Game/Data/S_Event` _returnvalue))
      (set `local.LocalLeftToBuy` _items_num)
      (set `local.LocalMustHaves` (`KismetArrayLibrary.Array_Length` _musthave_items_id))
      (set `local.LocalMaybe` (`KismetArrayLibrary.Array_Length` _maybe_items_id))
      ;[0.01938 0.01938 0.01938] while people are willing to buy
      (while (>= (`local.LocalLeftToBuy`) 0)
        ;[0.01938 0.01938 0.01938] if there is still can be a must-have item
        (if (> (`local.LocalMustHaves`) 0)
          (bind _output (`|GetArrayItem` _musthave_items_id (- (`local.LocalMustHaves`) 1)))
          (bind (_index _bfound) (`/Game/Modules/Inventory/AC_InventorySystem.Find Item` (`self.SellInventory`) _output))
          ;[0.01938 0.01938 0.01938] if we found a must-have item
          (if _bfound
            (bind (_data_isingredient _data_ispotion _data_name _data_description _data_thumbnail _data_class _data_maxstacksize _data_cost) (break `/Game/Modules/Inventory/S_Item` (`/Game/Modules/Inventory/AC_InventorySystem.Get Item Data` (`self.SellInventory`) _output)))
            (`self.Add Coins` _data_cost)
            (`self.Remove Item` _index true)
            (`/Engine/EditorBlueprintResources/StandardMacros.DecrementInt` (`local.LocalMustHaves`)
              (:`  `
                (`/Engine/EditorBlueprintResources/StandardMacros.DecrementInt` (`local.LocalLeftToBuy`))))
            (else
              (`/Engine/EditorBlueprintResources/StandardMacros.DecrementInt` (`local.LocalMustHaves`))))
          (else
            ;[0.01938 0.01938 0.01938] if there can be maybe-items
            (if (> (`local.LocalMaybe`) 0)
              (bind _output_2 (`|GetArrayItem` _maybe_items_id (- (`local.LocalMaybe`) 1)))
              (bind (_index_2 _bfound_2) (`/Game/Modules/Inventory/AC_InventorySystem.Find Item` (`self.SellInventory`) _output_2))
              ;[0.01938 0.01938 0.01938] if there is a maybe-item
              (if _bfound_2
                (bind (_data_isingredient_2 _data_ispotion_2 _data_name_2 _data_description_2 _data_thumbnail_2 _data_class_2 _data_maxstacksize_2 _data_cost_2) (break `/Game/Modules/Inventory/S_Item` (`/Game/Modules/Inventory/AC_InventorySystem.Get Item Data` (`self.SellInventory`) _output_2)))
                (`self.Add Coins` _data_cost_2)
                (`self.Remove Item` _index_2 true)
                (`/Engine/EditorBlueprintResources/StandardMacros.DecrementInt` (`local.LocalMaybe`)
                  (:`  `
                    (`/Engine/EditorBlueprintResources/StandardMacros.DecrementInt` (`local.LocalLeftToBuy`))))
                (else
                  (`/Engine/EditorBlueprintResources/StandardMacros.DecrementInt` (`local.LocalMaybe`))))
              (else
                (return))))))
      (return))))