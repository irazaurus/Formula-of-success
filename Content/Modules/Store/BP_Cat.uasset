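; BP_Cat is an interactable store actor that opens the store interface when a character interacts with it.
; Interact stores the character reference, hides the interaction prompt widget and blends the first player's view to the cat over a short ease-in.
; It then flags the character's main widget as camera-switched and in-store, switches it to the store tab and plays an interact sound.
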(event `/Game/Modules/Interact/BPI_Interact.Interact`
  (params (CharacterRef :type "/Game/Modules/Core/ThirdPersonControl/Blueprints/BP_ThirdPersonCharacter Object Reference"))
  (bind _mainwidget (`/Game/Modules/Core/ThirdPersonControl/Blueprints/BP_ThirdPersonCharacter.MainWidget` (`self.CharacterRef`)))
  (set `self.CharacterRef` CharacterRef)
  (`SceneComponent.SetHiddenInGame` (`self.WidgetInteract`) true false)
  (`PlayerController.SetViewTargetWithBlend` (`GameplayStatics.GetPlayerController` 0) self 0.3 "VTBlend_EaseIn" 0.0 false)
  (set `/Game/Modules/UI/WBP_PlayerView.bCameraSwitched` true _mainwidget)
  (set `/Game/Modules/UI/WBP_PlayerView.bInStore` true _mainwidget)
  (`/Game/Modules/UI/WBP_PlayerView.Change Tab` _mainwidget 5)
  (`GameplayStatics.PlaySound2D` (`self.InteractSound`) 1.0 1.0 0.0 null null))

(fn `UserConstructionScript`
  (`parent.UserConstructionScript`))