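; Bird AI character that drops a feather and flies away when it perceives the player.
; AI perception updates for the player pass only when the sense class is not AISenseConfig_Hearing, although the comment describes hearing.
; The reaction spawns BP_Feather just ahead once, sets the blackboard's hasNoticedPlayer flag and switches CharacterMovement to Flying.
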(event `Fly`
  (`CharacterMovementComponent.SetMovementMode` (`self.CharacterMovement`) "MOVE_Flying" 0))

(event `self.AIPerception.OnTargetPerceptionUpdated`
  (params (Actor :type "Actor Object Reference") (Stimulus :type "AIStimulus Structure"))
  (if (== (`GameplayStatics.GetPlayerCharacter` 0) Actor)
    ;[0.4531 0.4531 0.4531] if it hears the player
    (bind _returnvalue (`AIPerceptionSystem.GetSenseClassForStimulus` Stimulus))
    (if (not (== _returnvalue "/Script/AIModule.AISenseConfig_Hearing"))
      ;[1 1 1] spawn feather
      (if (not (`self.bSpawned`))
        (set `self.bSpawned` true)
        (`|SpawnActorFromClass` "/Game/Modules/Items/BP_Feather.BP_Feather_C" (`KismetMathLibrary.MakeTransform` (+ (`self.K2_GetActorLocation`) (* (`self.GetActorForwardVector`) 10.0))) "Undefined" "MultiplyWithRoot" null null))
      ;[0.3438 0.3438 0.3438] fly away
      (`BlackboardComponent.SetValueAsBool` (`AIBlueprintHelperLibrary.GetBlackboard` (`AIBlueprintHelperLibrary.GetAIController` self)) "hasNoticedPlayer" true)
      (`self.Fly`))))

(fn `UserConstructionScript`
  (`parent.UserConstructionScript`))