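; Teleport circle interactable that sends the interacting character from the cave (CaveMap1) to the Forest level.
; On Interact it plays a sound, starts a non-blocking stream load of Forest, moves the character to a hard-coded location and turns it around, then unloads CaveMap1.
; It also clears the Forest AI message through the GameInstance and GameState before the move and respawns it afterwards.
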(event `self.Interact`
  (params (CharacterRef :type "/Game/Modules/Core/ThirdPersonControl/Blueprints/BP_ThirdPersonCharacter Object Reference"))
  (message `/Game/Modules/Core/SaveGame/BPI_SaveGame.SaveForestAI` (`GameplayStatics.GetGameInstance`) false)
  (message `/Game/Modules/Core/ThirdPersonControl/Blueprints/BPI_GameState.Clear Forest AI` (`GameplayStatics.GetGameState`))
  (message `/Game/Modules/Effects/BPI_MusicPlayer.PlaySound` (`GameplayStatics.GetGameInstance`) (`self.InteractSound`) 1.0 0.0)
  (`GameplayStatics.LoadStreamLevel` "Forest" true)
  (`self.K2_SetActorLocation` CharacterRef (13880.0 -21890.0 410.0) false true)
  (`self.K2_AddActorWorldRotation` CharacterRef (struct :`Yaw` 180.0) false false)
  (message `/Game/Modules/Core/ThirdPersonControl/Blueprints/BPI_GameState.Spawn Forest AI` (`GameplayStatics.GetGameState`) true)
  (`GameplayStatics.UnloadStreamLevel` "CaveMap1"))

(fn `UserConstructionScript`
  (`parent.UserConstructionScript`))