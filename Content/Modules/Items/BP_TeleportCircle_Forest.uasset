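; Interactable teleport circle that moves a character from the TownMap level to the Forest level.
; On Interact it plays a sound, starts a non-blocking stream load of Forest and notifies the GameState of the level change.
; It then moves the character to a hardcoded location, rotates them 180 degrees and unloads TownMap, without waiting for the load to finish.
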(event `self.Interact`
  (params (CharacterRef :type "/Game/Modules/Core/ThirdPersonControl/Blueprints/BP_ThirdPersonCharacter Object Reference"))
  (`GameplayStatics.PlaySound2D` (`self.InteractSound`) 1.0 1.0 0.0 null null)
  (`GameplayStatics.LoadStreamLevel` "Forest" true)
  (message `/Game/Modules/Core/ThirdPersonControl/Blueprints/BPI_GameState.Call OnLevelChanged` (`GameplayStatics.GetGameState`) "Forest")
  (`self.K2_SetActorLocation` CharacterRef (23999.0 -19674.0 757.0) false false)
  (`self.K2_AddActorWorldRotation` CharacterRef (struct :`Yaw` 180.0) false false)
  (`GameplayStatics.UnloadStreamLevel` "TownMap"))

(fn `UserConstructionScript`
  (`parent.UserConstructionScript`))