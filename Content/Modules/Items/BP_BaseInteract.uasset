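; BP_BaseInteract is a base Blueprint for interactable items that show an interaction prompt when something enters their trigger box.
; On BeginPlay it looks up the ACItemComponent's ItemID row in its data table and creates a WB_InteractMessage with the row's name for the WidgetInteract component.
; InteractBox overlaps show or hide that widget, without filtering the overlapping actor.
; The Interact event forwards the character reference to ACItemComponent, which handles the interaction.
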(event `self.ReceiveBeginPlay`
  (bind (_itemid_datatable _itemid_rowname) (break `DataTableRowHandle` (`/Game/Modules/Inventory/AC_ItemComponent.ItemID` (`self.AC_ItemComponent`))))
  (bind _returnvalue (`|GetDataTableRow` _itemid_datatable _itemid_rowname)
    (:`then`
      (bind _returnvalue_2 (`|CreateWidget` "/Game/Modules/Interact/WB_InteractMessage.WB_InteractMessage_C" null (`.Name_3_500006F34D6F0976789AC592F8AEF5A8` (break `/Game/Modules/Inventory/S_Item` _returnvalue))))
      (`WidgetComponent.SetWidget` (`self.WidgetInteract`) _returnvalue_2))))

(event `/Game/Modules/Interact/BPI_Interact.Interact`
  (params (CharacterRef :type "/Game/Modules/Core/ThirdPersonControl/Blueprints/BP_ThirdPersonCharacter Object Reference"))
  (`/Game/Modules/Inventory/AC_ItemComponent.Interact` (`self.AC_ItemComponent`) CharacterRef))

(event `self.InteractBox.OnComponentBeginOverlap`
  (params (OverlappedComponent :type "PrimitiveComponent Object Reference") (OtherActor :type "Actor Object Reference") (OtherComp :type "PrimitiveComponent Object Reference") (OtherBodyIndex :type Integer) (bFromSweep :type Boolean) (SweepResult :type "HitResult Structure (by ref)"))
  (`SceneComponent.SetHiddenInGame` (`self.WidgetInteract`) false false))

(event `self.InteractBox.OnComponentEndOverlap`
  (params (OverlappedComponent :type "PrimitiveComponent Object Reference") (OtherActor :type "Actor Object Reference") (OtherComp :type "PrimitiveComponent Object Reference") (OtherBodyIndex :type Integer))
  (`SceneComponent.SetHiddenInGame` (`self.WidgetInteract`) true false))

(fn `UserConstructionScript`)