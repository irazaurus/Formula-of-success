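; An interactable teleport circle that sends the interacting character from the room map to the town map.
; On Interact it plays a sound, streams in TownMap without blocking and notifies the GameState of the level change.
; It then moves the character to a hardcoded town location and streams out RoomMap.
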(event `self.Interact`
  (params (CharacterRef :type "/Game/Modules/Core/ThirdPersonControl/Blueprints/BP_ThirdPersonCharacter Object Reference"))
  (`GameplayStatics.PlaySound2D` (`self.InteractSound`) 1.0 1.0 0.0 null null)
  (`GameplayStatics.LoadStreamLevel` "TownMap" true)
  (message `/Game/Modules/Core/ThirdPersonControl/Blueprints/BPI_GameState.Call OnLevelChanged` (`GameplayStatics.GetGameState`) "TownMap")
  (`self.K2_SetActorLocation` CharacterRef (165.0 -9267.0 2988.0) false false)
  (`GameplayStatics.UnloadStreamLevel` "RoomMap"))

(fn `UserConstructionScript`
  (`parent.UserConstructionScript`))