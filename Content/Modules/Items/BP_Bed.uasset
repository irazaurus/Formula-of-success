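; BP_Bed is an interactable bed that moves the game on to a new day.
; On Interact, it gets the new-day and current-day messages from the GameState and shows a WBP_NewDay widget with the day.
; An "End" message opens the end-game tab on the character's main widget.
; Any other message is passed to the character's AC_StoreComponent to update stock, followed by an interaction sound.
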(event `/Game/Modules/Interact/BPI_Interact.Interact`
  (params (CharacterRef :type "/Game/Modules/Core/ThirdPersonControl/Blueprints/BP_ThirdPersonCharacter Object Reference"))
  (bind _prevday (message `/Game/Modules/Core/ThirdPersonControl/Blueprints/BPI_GameState.NewDay` (`GameplayStatics.GetGameState`)))
  (bind _day (message `/Game/Modules/Core/ThirdPersonControl/Blueprints/BPI_GameState.GetDay` (`GameplayStatics.GetGameState`)))
  (bind _returnvalue (`|CreateWidget` "/Game/Modules/UI/WBP_NewDay.WBP_NewDay_C" null _day))
  (`UserWidget.AddToViewport` _returnvalue 0)
  (if (== _prevday "End")
    (`/Game/Modules/UI/WBP_PlayerView.EndGameTab` (`/Game/Modules/Core/ThirdPersonControl/Blueprints/BP_ThirdPersonCharacter.MainWidget` CharacterRef) false)
    (else
      (`/Game/Modules/Store/AC_StoreComponent.Update Stock` (`self.GetComponentByClass` CharacterRef "/Game/Modules/Store/AC_StoreComponent.AC_StoreComponent_C") _prevday)
      (`GameplayStatics.PlaySound2D` (`self.InteractSound`) 1.0 1.0 0.0 null null))))

(fn `UserConstructionScript`
  (`parent.UserConstructionScript`))