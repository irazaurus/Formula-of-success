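; BP_TeleportCircle_Room is an interactable teleport circle that sends the interacting character from TownMap to RoomMap.
; On Interact it starts a non-blocking stream load of RoomMap, notifies the GameState of the level change and plays a sound through the GameInstance.
; It then moves the character to a hardcoded location and unloads TownMap, without waiting for the load to finish.
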(event `/Game/Modules/Interact/BPI_Interact.Interact`
  (params (CharacterRef :type "/Game/Modules/Core/ThirdPersonControl/Blueprints/BP_ThirdPersonCharacter Object Reference"))
  (`GameplayStatics.LoadStreamLevel` "RoomMap" true)
  (message `/Game/Modules/Core/ThirdPersonControl/Blueprints/BPI_GameState.Call OnLevelChanged` (`GameplayStatics.GetGameState`) "RoomMap")
  (message `/Game/Modules/Effects/BPI_MusicPlayer.PlaySound` (`GameplayStatics.GetGameInstance`) (`self.InteractSound`) 1.0 0.0)
  (`self.K2_SetActorLocation` CharacterRef (-430.0 880.0 222.0) false false)
  (`GameplayStatics.UnloadStreamLevel` "TownMap"))

(fn `UserConstructionScript`
  (`parent.UserConstructionScript`))